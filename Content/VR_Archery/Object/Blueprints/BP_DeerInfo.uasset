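; VR archery info point, named for deer, that shows a pop-up text widget when a motion controller enters its box and hides it on exit.
; BeginPlay copies a non-empty UIText into the PopUp_UI widget and sets its text visibility from IsShowContinue, which also disables overlap toggling when true.
; While the text is visible, Tick turns the widget on yaw only to face the player camera.
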(event `self.Box.OnComponentBeginOverlap`
  (params (OverlappedComponent :type "PrimitiveComponent Object Reference") (OtherActor :type "Actor Object Reference") (OtherComp :type "PrimitiveComponent Object Reference") (OtherBodyIndex :type Integer) (bFromSweep :type Boolean) (SweepResult :type "HitResult Structure (by ref)"))
  ;[1 1 1] Show and Hide UI
  (if (not (`self.IsShowContinue`))
    (cast `/Game/VR_Archery/Characters/VRPawn/BP_MotionController` OtherActor)
    (bind _aspop_up_ui (cast `/Game/VR_Archery/UI/PopUp_UI` (`WidgetComponent.GetUserWidgetObject` (`self.Widget`))))
    (`/Game/VR_Archery/UI/PopUp_UI.ShowPopUp` _aspop_up_ui)))

(event `self.Box.OnComponentEndOverlap`
  (params (OverlappedComponent :type "PrimitiveComponent Object Reference") (OtherActor :type "Actor Object Reference") (OtherComp :type "PrimitiveComponent Object Reference") (OtherBodyIndex :type Integer))
  ;[1 1 1] Show and Hide UI
  (if (not (`self.IsShowContinue`))
    (cast `/Game/VR_Archery/Characters/VRPawn/BP_MotionController` OtherActor)
    (bind _aspop_up_ui (cast `/Game/VR_Archery/UI/PopUp_UI` (`WidgetComponent.GetUserWidgetObject` (`self.Widget`))))
    (`/Game/VR_Archery/UI/PopUp_UI.HidePopUp` _aspop_up_ui)))

(event `self.ReceiveBeginPlay`
  (`|ExecutionSequence`
    (:`then_0`
      ;[1 1 1] Set UI Text
      (if (not (`KismetTextLibrary.TextIsEmpty` (`self.UI Text`)))
        (bind _aspop_up_ui (cast `/Game/VR_Archery/UI/PopUp_UI` (`WidgetComponent.GetUserWidgetObject` (`self.Widget`))))
        (set `/Game/VR_Archery/UI/PopUp_UI.Text` (`self.UI Text`) _aspop_up_ui)))
    (:`then_1`
      ;[1 1 1] Set Text visibility
      (bind _aspop_up_ui_2 (cast `/Game/VR_Archery/UI/PopUp_UI` (`WidgetComponent.GetUserWidgetObject` (`self.Widget`))))
      (`/Game/VR_Archery/UI/PopUp_UI.SetShowText` _aspop_up_ui_2 (`self.IsShowContinue`)))))

(event `self.ReceiveTick`
  (params (DeltaSeconds :type "Float (single-precision)"))
  (bind _aspop_up_ui (cast `/Game/VR_Archery/UI/PopUp_UI` (`WidgetComponent.GetUserWidgetObject` (`self.Widget`))))
  (if (`/Game/VR_Archery/UI/PopUp_UI.GetVisibilityText` _aspop_up_ui)
    (`self.UpdatePopUpFacing`)))

(fn `UpdatePopUpFacing`
  (bind (_returnvalue_roll _returnvalue_pitch _returnvalue_yaw) (`KismetMathLibrary.BreakRotator` (`KismetMathLibrary.FindLookAtRotation` (`SceneComponent.K2_GetComponentLocation` (`self.Widget`)) (`PlayerCameraManager.GetCameraLocation` (`GameplayStatics.GetPlayerCameraManager` 0)))))
  (`SceneComponent.K2_SetWorldRotation` (`self.Widget`) (`KismetMathLibrary.MakeRotator` 0.0 0.0 _returnvalue_yaw) false false))

(fn `UserConstructionScript`)