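; BP_Target is a VR archery target that registers scoring hits and gives audio feedback.
; Its TargetHit event accepts only hits on the Target component, notifies GameMode_Archery of the score, then plays a sound at the actor root.
; The construction script applies a Color variable to the target's material and point light.
; PlaySound checks a PlayingSound flag but clears it immediately after starting playback, so it does not prevent overlapping sounds.
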(event `TargetHit`
  (params (HitLocation :type "Vector Structure") (ComponentHit :type "PrimitiveComponent Object Reference"))
  ;[1 1 1] Target hit
  (if (== ComponentHit (`self.Target`))
    (bind _asgame_mode_archery (cast `/Game/VR_Archery/Core/GameMode_Archery` (`GameplayStatics.GetGameMode`)))
    (`/Game/VR_Archery/Core/GameMode_Archery.PlayerHasScored` _asgame_mode_archery)
    (`self.PlaySound` "/Game/VR_Archery/Sounds/targetHit.targetHit" (`SceneComponent.K2_GetComponentLocation` (`self.DefaultSceneRoot`)))))

(fn `PlaySound`
  (params (Sound :type "SoundBase Object Reference") (SoundLocation :type "Vector Structure"))
  (if (not (`self.PlayingSound`))
    (set `self.PlayingSound` true)
    (`GameplayStatics.PlaySoundAtLocation` Sound SoundLocation (struct) 1.0 1.0 0.0 null null null)
    (set `self.PlayingSound` false)))

(fn `UserConstructionScript`
  (bind _color (`self.Color`))
  (`MeshComponent.SetVectorParameterValueOnMaterials` (`self.Target`) "Color" (`KismetMathLibrary.Conv_LinearColorToVector` _color))
  (`LightComponent.SetLightColor` (`self.PointLight`) _color true))