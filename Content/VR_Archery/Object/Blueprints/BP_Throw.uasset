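; BP_Throw is a VR throwable, apparently a knife, that can be picked up, thrown and stuck into targets.
; Pickup attaches it with physics off; Drop re-enables physics, stores the release velocity and starts a 60 Hz timer.
; During flight it aligns to that velocity, adds force along it and sphere-traces ahead to notify BP_Target.
; Hitting a target or static mesh actor freezes it and starts a short lifespan.
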(event `/Game/VR_Archery/Object/Blueprints/PickupActorInterface_Archery.Pickup`
  (params (AttachTo :type "SceneComponent Object Reference"))
  ;[1 1 1] Pick up this
  (`PrimitiveComponent.SetSimulatePhysics` (`self.StaticMeshComponent`) false)
  (`SceneComponent.K2_AttachToComponent` (`self.K2_GetRootComponent`) AttachTo "None" "SnapToTarget" "SnapToTarget" "KeepWorld" false)
  (`SceneComponent.K2_SetRelativeLocation` (`self.StaticMeshComponent`) (-3.0 -1.0 0.0) false false)
  (`self.PlaySound` "/Game/VR_Archery/Sounds/grabKnife.grabKnife" (`SceneComponent.K2_GetComponentLocation` (`self.StaticMeshComponent`))))

(event `/Game/VR_Archery/Object/Blueprints/PickupActorInterface_Archery.Drop`
  ;[1 1 1] Drop this
  (`PrimitiveComponent.SetSimulatePhysics` (`self.StaticMeshComponent`) true)
  (`self.K2_DetachFromActor` "KeepWorld" "KeepWorld" "KeepWorld")
  (set `self.ThrowVelocity` (`self.GetVelocity`))
  (bind _returnvalue (`KismetSystemLibrary.K2_SetTimerDelegate` (`|CreateDelegate` :!event `AdjustRotationFromThrow`) (/ 1.0 60.0) true))
  (set `self.RotationTimer` _returnvalue)
  (set `self.IsThrowing` true))

(event `AdjustRotationFromThrow`
  (bind _returnvalue (`self.K2_GetActorLocation`))
  (bind (_returnvalue_roll _returnvalue_pitch _returnvalue_yaw) (`KismetMathLibrary.BreakRotator` (`KismetMathLibrary.FindLookAtRotation` _returnvalue (+ _returnvalue (`self.ThrowVelocity`)))))
  ;[1 1 1] Throw Rotation Set
  (`self.K2_SetActorRotation` (`KismetMathLibrary.MakeRotator` _returnvalue_roll (- _returnvalue_pitch 90.0) _returnvalue_yaw))
  (`PrimitiveComponent.AddForce` (`self.StaticMeshComponent`) (* (`self.ThrowVelocity`) 10.0) "None" true)
  (`self.CheckIfHitSomething`))

(event `CheckIfHitSomething`
  (bind _arrow (`self.Arrow`))
  (bind _returnvalue (`SceneComponent.K2_GetComponentLocation` _arrow))
  ;[1 1 1] Check Hit Something
  (bind _outhit (`KismetSystemLibrary.SphereTraceSingle` _returnvalue (+ _returnvalue (* (`SceneComponent.GetForwardVector` _arrow) 20.0)) 5.0 "TraceTypeQuery1"))
  (bind (_bblockinghit _binitialoverlap _time _distance _location _impactpoint _normal _impactnormal _physmat _hitactor _hitcomponent) (`GameplayStatics.BreakHitResult` _outhit))
  (if _bblockinghit
    (bind _asbp_target (cast `/Game/VR_Archery/Object/Blueprints/BP_Target` _hitactor))
    (`/Game/VR_Archery/Object/Blueprints/BP_Target.TargetHit` _asbp_target _impactpoint _hitcomponent)
    (`self.StopMotion`)))

(event `StopMotion`
  ;[1 1 1] Stop Actor
  (`PrimitiveComponent.SetSimulatePhysics` (`self.StaticMeshComponent`) false)
  (`KismetSystemLibrary.K2_PauseTimerHandle` (`self.RotationTimer`))
  (set `self.IsThrowing` false)
  (`self.SetLifeSpan` 5.0))

(event `self.StaticMeshComponent.OnComponentHit`
  (params (HitComponent :type "PrimitiveComponent Object Reference") (OtherActor :type "Actor Object Reference") (OtherComp :type "PrimitiveComponent Object Reference") (NormalImpulse :type "Vector Structure") (Hit :type "HitResult Structure (by ref)"))
  ;[1 1 1] Hit When Throwing(Not Target)
  (if (`self.IsThrowing`)
    (cast `StaticMeshActor` OtherActor)
    (`self.StopMotion`)))

(fn `PlaySound`
  (params (Sound :type "SoundBase Object Reference") (SoundLocation :type "Vector Structure"))
  (if (not (`self.PlayingSound`))
    (set `self.PlayingSound` true)
    (`GameplayStatics.PlaySoundAtLocation` Sound SoundLocation (struct) 1.0 1.0 0.0 null null null)
    (set `self.PlayingSound` false)))

(fn `UserConstructionScript`
  (`parent.UserConstructionScript`))