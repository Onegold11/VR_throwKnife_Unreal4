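; Grabbable physics object for VR archery that can be held, dropped or pulled through the air toward the player's hand.
; Pickup disables physics and attaches it to the given component, while Drop re-enables physics and detaches it.
; ToPlayer plays a sound and starts a 60 Hz timer for the launch.
; The launch repeatedly applies a suggested projectile velocity as acceleration toward the hand, pausing the timer once near the player.
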(event `/Game/VR_Archery/Object/Blueprints/PickupActorInterface_Archery.Pickup`
  (params (AttachTo :type "SceneComponent Object Reference"))
  ;[1 1 1] Pick up event
  (`PrimitiveComponent.SetSimulatePhysics` (`self.StaticMeshComponent`) false)
  (`SceneComponent.K2_AttachToComponent` (`self.K2_GetRootComponent`) AttachTo "None" "KeepWorld" "KeepWorld" "KeepWorld" false))

(event `/Game/VR_Archery/Object/Blueprints/PickupActorInterface_Archery.Drop`
  ;[1 1 1] Drop event
  (`PrimitiveComponent.SetSimulatePhysics` (`self.StaticMeshComponent`) true)
  (`self.K2_DetachFromActor` "KeepWorld" "KeepWorld" "KeepWorld"))

(event `/Game/VR_Archery/Object/Blueprints/GravityActorInterface_Archery.ToPlayer`
  (params (Hand :type "/Game/VR_Archery/Characters/VRPawn/BP_MotionController Object Reference") (Player :type "/Game/VR_Archery/Characters/VRPawn/MotionControllerPawn_Archery Object Reference"))
  ;[1 1 1] To Player event
  (if (not (`self.IsLaunching`))
    (set `self.IsLaunching` true)
    (set `self.Hand` Hand)
    (set `self.Player` Player)
    (bind _returnvalue (`KismetSystemLibrary.K2_SetTimerDelegate` (`|CreateDelegate` :!event `LaunchActorToPlayer`) (/ 1.0 60.0) true))
    (set `self.LaunchTimer` _returnvalue)
    (`GameplayStatics.PlaySoundAtLocation` "/Game/VR_Archery/Sounds/targetLaunch.targetLaunch" (`SceneComponent.K2_GetComponentLocation` (`self.StaticMeshComponent`)) (struct) 1.0 1.0 0.0 null null null)))

(event `LaunchActorToPlayer`
  ;[1 1 1] Launch Actor to Player
  (bind _tossvelocity (`GameplayStatics.BlueprintSuggestProjectileVelocity` (`SceneComponent.K2_GetComponentLocation` (`self.StaticMeshComponent`)) (`SceneComponent.K2_GetComponentLocation` (`/Game/VR_Archery/Characters/VRPawn/BP_MotionController.HandMesh` (`self.Hand`))) 1000.0 0.0 "DoNotTrace" 10.0))
  (`PrimitiveComponent.AddForce` (`self.StaticMeshComponent`) _tossvelocity "None" true)
  (if (<= (`self.GetDistanceTo` (`self.Player`)) 150.0)
    (`KismetSystemLibrary.K2_PauseTimerHandle` (`self.LaunchTimer`))
    (set `self.IsLaunching` false)))

(fn `UserConstructionScript`)